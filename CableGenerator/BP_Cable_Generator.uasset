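; BP_Cable_Generator is a construction-script actor that builds a cable from spline mesh components along an editable spline.
; StretchMeshMethod stretches one mesh per point segment; otherwise segments repeat at mesh Z length times a resolution factor, avoiding stretched UVs.
; Options set thickness, curve type, materials, floor offset and end-tangent correction, with start and end cap meshes placed on top.
; Mesh-copy scattering and point-number labels exist but are unconnected.
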(fn `UserConstructionScript`
  (locals (SplineMeshRadius :type "Float (double-precision)" :default 1.0))
  (bind _endmesh (`self.EndMesh`))
  (bind _spline (`self.Spline`))
  (bind _spline_2 (`self.Spline`))
  (bind _splinemeshthickness (`self.SplineMeshThickness`))
  (bind _spline_3 (`self.Spline`))
  (bind _internalsplinemeshcomponent (`self.InternalSplineMeshComponent`))
  (bind _loopcountersplinemesh (`self.LoopCounterSplineMesh`))
  (bind _spline_4 (`self.Spline`))
  (bind _spline_5 (`self.Spline`))
  (bind _internalsplinemeshcomponent_2 (`self.InternalSplineMeshComponent`))
  (bind _splinemeshmat (`self.SplineMeshMat`))
  (bind (_endmeshrotation_roll _endmeshrotation_pitch _endmeshrotation_yaw) (`KismetMathLibrary.BreakRotator` (`self.EndMeshRotation`)))
  (bind _spline_6 (`self.Spline`))
  (bind _startmesh (`self.StartMesh`))
  (bind _spline_7 (`self.Spline`))
  (bind _loopcountersplinemesh_2 (`self.LoopCounterSplineMesh`))
  (bind _spline_8 (`self.Spline`))
  (bind (_startmeshrotation_roll _startmeshrotation_pitch _startmeshrotation_yaw) (`KismetMathLibrary.BreakRotator` (`self.StartMeshRotation`)))
  (bind _internalsplinemeshcomponent_3 (`self.InternalSplineMeshComponent`))
  (bind _splinemeshmat_2 (`self.SplineMeshMat`))
  (bind _endmeshmat (`self.EndMeshMat`))
  (bind _startmeshmat (`self.StartMeshMat`))
  (bind _splinemeshthickness_2 (`self.SplineMeshThickness`))
  (bind (_returnvalue_x _returnvalue_y) (`KismetMathLibrary.BreakVector` (`SplineComponent.GetTangentAtSplinePoint` (`self.Spline`) 0 "Local")))
  (bind (_returnvalue_x_2 _returnvalue_y_2) (`KismetMathLibrary.BreakVector` (`SplineComponent.GetTangentAtSplinePoint` (`self.Spline`) 0 "Local")))
  (bind (_returnvalue_x_3 _returnvalue_y_3) (`KismetMathLibrary.BreakVector` (`SplineComponent.GetTangentAtSplinePoint` (`self.Spline`) 0 "Local")))
  (bind (_location _tangent) (`SplineComponent.GetLocationAndTangentAtSplinePoint` _spline_3 _loopcountersplinemesh "Local"))
  (bind _returnvalue (`KismetMathLibrary.MakeVector2D` _splinemeshthickness _splinemeshthickness))
  (bind _returnvalue_2 (* _loopcountersplinemesh_2 (`self.Input_mesh_height`)))
  (bind (_returnvalue_roll _returnvalue_pitch _returnvalue_yaw) (`KismetMathLibrary.BreakRotator` (`SplineComponent.GetRotationAtSplinePoint` _spline_6 0 "Local")))
  (bind (_returnvalue_x_4 _returnvalue_y_4) (`KismetMathLibrary.BreakVector` (`SplineComponent.GetTangentAtSplinePoint` (`self.Spline`) 0 "Local")))
  (bind _returnvalue_3 (`KismetMathLibrary.MakeVector2D` _splinemeshthickness_2 _splinemeshthickness_2))
  (bind _returnvalue_4 (`SplineComponent.GetNumberOfSplinePoints` _spline))
  (bind _returnvalue_5 (- (`SplineComponent.GetNumberOfSplinePoints` _spline_2) 1))
  (bind _returnvalue_6 (- (`SplineComponent.GetNumberOfSplinePoints` _spline_4) 1))
  (bind _returnvalue_7 (- (`SplineComponent.GetNumberOfSplinePoints` _spline_5) 1))
  (bind (_location_2 _tangent_2) (`SplineComponent.GetLocationAndTangentAtSplinePoint` _spline_3 (+ _loopcountersplinemesh 1) "Local"))
  (bind (_returnvalue_x_5 _returnvalue_y_5 _returnvalue_z) (`KismetMathLibrary.BreakVector` (`SplineComponent.GetTangentAtDistanceAlongSpline` _spline_7 _returnvalue_2 "Local")))
  (bind _returnvalue_8 (* (+ _loopcountersplinemesh_2 1) (`self.Input_mesh_height`)))
  (bind _returnvalue_9 (- (`SplineComponent.GetNumberOfSplinePoints` _spline_8) 1))
  (bind (_returnvalue_roll_2 _returnvalue_pitch_2 _returnvalue_yaw_2) (`KismetMathLibrary.BreakRotator` (`SplineComponent.GetRotationAtSplinePoint` _spline _returnvalue_4 "World")))
  (bind (_returnvalue_x_6 _returnvalue_y_6) (`KismetMathLibrary.BreakVector` (`SplineComponent.GetTangentAtSplinePoint` (`self.Spline`) _returnvalue_5 "Local")))
  (bind (_returnvalue_x_7 _returnvalue_y_7) (`KismetMathLibrary.BreakVector` (`SplineComponent.GetTangentAtSplinePoint` (`self.Spline`) _returnvalue_6 "Local")))
  (bind (_returnvalue_x_8 _returnvalue_y_8 _returnvalue_z_2) (`KismetMathLibrary.BreakVector` (`SplineComponent.GetTangentAtSplinePoint` (`self.Spline`) _returnvalue_7 "Local")))
  (bind (_returnvalue_x_9 _returnvalue_y_9 _returnvalue_z_3) (`KismetMathLibrary.BreakVector` (`SplineComponent.GetTangentAtDistanceAlongSpline` _spline_7 _returnvalue_8 "Local")))
  (bind (_returnvalue_x_10 _returnvalue_y_10 _returnvalue_z_4) (`KismetMathLibrary.BreakVector` (`SplineComponent.GetTangentAtSplinePoint` (`self.Spline`) _returnvalue_9 "Local")))
  (`StaticMeshComponent.SetStaticMesh` (`self.SplineMesh`) (`self.SplineMeshInput`))
  (`StaticMeshComponent.SetStaticMesh` (`self.EndMesh`) (`self.EndMeshInput`))
  (`StaticMeshComponent.SetStaticMesh` (`self.StartMesh`) (`self.StartMeshInput`))
  (bind _output_get (set `local.SplineMeshRadius` (.x (`.Max` (`StaticMeshComponent.GetLocalBounds` (`self.SplineMesh`))))))
  (`self.Set Input mesh height` (`self.SplineMeshResolution`))
  ;[1 1 1] Floor Autocorrect
  (if (`self.FloorAutocorrect`)
    (for _index (range (`self.FloorAutocorrectStart`) (+ (- (- (`SplineComponent.GetNumberOfSplinePoints` (`self.Spline`)) 1) (`self.FloorAutocorrectEnd`)) 1))
      (`SplineComponent.SetLocationAtSplinePoint` (`self.Spline`) _index (`self.Add Z Value To Vector` (`SplineComponent.GetLocationAtSplinePoint` (`self.Spline`) _index "Local") (* (`local.SplineMeshRadius`) (`self.SplineMeshThickness`))) "Local" true)))
  (if (`self.StretchMeshMethod`)
    ;[1 1 1] Generate Cable Stretched UVs
    (for _index_2 (range (+ (- (`SplineComponent.GetNumberOfSplinePoints` (`self.Spline`)) 2) 1))
      ;;[1 1 1] Set Spline Point Type
      (`SplineComponent.SetSplinePointType` (`self.Spline`) _index_2 (`self.CurveType`) true)
      (set `self.LoopCounterSplineMesh` _index_2)
      (bind _returnvalue_10 (`AddComponent|NODE_AddSplineMeshComponent-1`))
      (bind _output_get_2 (set `self.InternalSplineMeshComponent` _returnvalue_10))
      ;;[1 1 1] Set Cable Thickness
      (`SplineMeshComponent.SetEndScale` _internalsplinemeshcomponent _returnvalue_3 true)
      (`SplineMeshComponent.SetStartScale` _internalsplinemeshcomponent _returnvalue_3 true)
      (`StaticMeshComponent.SetStaticMesh` _output_get_2 (`StaticMeshComponent.StaticMesh` (`self.SplineMesh`)))
      (`SceneComponent.K2_AttachTo` (`self.InternalSplineMeshComponent`) (`self.Spline`) "None" "KeepRelativeOffset" true)
      ;;[1 1 1] Materialslots SplineMesh
      (`KismetArrayLibrary.Array_Resize` _splinemeshmat (`PrimitiveComponent.GetNumMaterials` _internalsplinemeshcomponent_2))
      (for (_array_element _array_index) _splinemeshmat
        (`PrimitiveComponent.SetMaterial` _internalsplinemeshcomponent_2 _array_index _array_element)
        (if (`self.StartEndCorrectHorizontal`)
          ;[1 1 1] Start End Spline Tangent Correction
          (`SplineComponent.SetTangentAtSplinePoint` (`self.Spline`) 0 (`KismetMathLibrary.MakeVector` _returnvalue_x _returnvalue_y) "Local" true)
          (`SplineComponent.SetTangentAtSplinePoint` _spline_2 _returnvalue_5 (`KismetMathLibrary.MakeVector` _returnvalue_x_6 _returnvalue_y_6) "Local" true)
          (elif (`self.EndCorrectVertical`)
            ;[1 1 1] Start End Spline Tangent Correction
            (`SplineComponent.SetTangentAtSplinePoint` (`self.Spline`) 0 (`KismetMathLibrary.MakeVector` _returnvalue_x_4 _returnvalue_y_4) "Local" true)
            (`SplineComponent.SetTangentAtSplinePoint` _spline_8 _returnvalue_9 (`KismetMathLibrary.MakeVector` 0.0 0.0 _returnvalue_z_4) "Local" true)))
        (`SplineMeshComponent.SetStartAndEnd` (`self.InternalSplineMeshComponent`) _location _tangent _location_2 _tangent_2 true)))
    (else
      ;[1 1 1] Generate Cable No Stretched UVs
      (for _index_3 (range (+ (`.ReturnValue` (`KismetMathLibrary.FMod` (`SplineComponent.GetSplineLength` (`self.Spline`)) (`self.Input_mesh_height`))) 1))
        ;;[1 1 1] Set Spline Point Type
        (`SplineComponent.SetSplinePointType` (`self.Spline`) _index_3 (`self.CurveType`) true)
        (set `self.LoopCounterSplineMesh` _index_3)
        (bind _returnvalue_11 (`AddComponent|NODE_AddSplineMeshComponent-0`))
        (bind _output_get_3 (set `self.InternalSplineMeshComponent` _returnvalue_11))
        ;;[1 1 1] Set Cable Thickness
        (`SplineMeshComponent.SetEndScale` _returnvalue_11 _returnvalue true)
        (`SplineMeshComponent.SetEndScale` (`self.InternalSplineMeshComponent`) _returnvalue true)
        (`SplineMeshComponent.SetStartScale` _returnvalue_11 _returnvalue true)
        (`SplineMeshComponent.SetStartScale` (`self.InternalSplineMeshComponent`) _returnvalue true)
        (`StaticMeshComponent.SetStaticMesh` _output_get_3 (`StaticMeshComponent.StaticMesh` (`self.SplineMesh`)))
        (`SceneComponent.K2_AttachTo` _returnvalue_11 (`self.Spline`) "None" "KeepRelativeOffset" true)
        ;;[1 1 1] Materialslots SplineMesh
        (`KismetArrayLibrary.Array_Resize` _splinemeshmat_2 (`PrimitiveComponent.GetNumMaterials` _internalsplinemeshcomponent_3))
        (for (_array_element_2 _array_index_2) _splinemeshmat_2
          (`PrimitiveComponent.SetMaterial` _internalsplinemeshcomponent_3 _array_index_2 _array_element_2)
          (`PrimitiveComponent.SetMaterial` (`self.SplineMesh`) _array_index_2 _array_element_2))
        (if (`self.StartEndCorrectHorizontal`)
          ;[1 1 1] Start End Spline Tangent Correction
          (`SplineComponent.SetTangentAtSplinePoint` (`self.Spline`) 0 (`KismetMathLibrary.MakeVector` _returnvalue_x_2 _returnvalue_y_2) "Local" true)
          (`SplineComponent.SetTangentAtSplinePoint` _spline_4 _returnvalue_6 (`KismetMathLibrary.MakeVector` _returnvalue_x_7 _returnvalue_y_7) "Local" true)
          (elif (`self.EndCorrectVertical`)
            ;[1 1 1] Start End Spline Tangent Correction
            (`SplineComponent.SetTangentAtSplinePoint` (`self.Spline`) 0 (`KismetMathLibrary.MakeVector` _returnvalue_x_3 _returnvalue_y_3) "Local" true)
            (`SplineComponent.SetTangentAtSplinePoint` _spline_5 _returnvalue_7 (`KismetMathLibrary.MakeVector` 0.0 0.0 _returnvalue_z_2) "Local" true)))
        ;;[1 1 1] Set Start End Points Splinemeshes
        (`SplineMeshComponent.SetStartAndEnd` (`self.InternalSplineMeshComponent`) (`SplineComponent.GetLocationAtDistanceAlongSpline` _spline_7 _returnvalue_2 "Local") (`KismetMathLibrary.MakeVector` _returnvalue_x_5 _returnvalue_y_5 _returnvalue_z) (`SplineComponent.GetLocationAtDistanceAlongSpline` _spline_7 _returnvalue_8 "Local") (`KismetMathLibrary.MakeVector` _returnvalue_x_9 _returnvalue_y_9 _returnvalue_z_3) true))))
  ;[1 1 1] Materialslots SplineMesh
  (`KismetArrayLibrary.Array_Resize` _startmeshmat (`PrimitiveComponent.GetNumMaterials` _startmesh))
  (for (_array_element_3 _array_index_3) _startmeshmat
    (`PrimitiveComponent.SetMaterial` _startmesh _array_index_3 _array_element_3))
  ;[1 1 1] Add StartMesh
  (`SceneComponent.K2_SetRelativeLocationAndRotation` _startmesh (`SplineComponent.GetLocationAtSplinePoint` _spline_6 0 "Local") (`KismetMathLibrary.MakeRotator` _startmeshrotation_roll (+ _returnvalue_pitch _startmeshrotation_pitch) (+ _returnvalue_yaw _startmeshrotation_yaw)) true false)
  ;[1 1 1] Materialslots SplineMesh
  (`KismetArrayLibrary.Array_Resize` _endmeshmat (`PrimitiveComponent.GetNumMaterials` _endmesh))
  (for (_array_element_4 _array_index_4) _endmeshmat
    (`PrimitiveComponent.SetMaterial` _endmesh _array_index_4 _array_element_4))
  ;[1 1 1] Add EndMesh
  (`SceneComponent.K2_SetRelativeLocationAndRotation` _endmesh (`SplineComponent.GetLocationAtSplinePoint` _spline _returnvalue_4 "Local") (`KismetMathLibrary.MakeRotator` _endmeshrotation_roll (+ _returnvalue_pitch_2 _endmeshrotation_pitch) (+ _returnvalue_yaw_2 _endmeshrotation_yaw)) false false))