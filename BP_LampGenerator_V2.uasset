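; Procedural hanging lamp generator that assembles socket, shade and cable in the Construction Script, with no runtime logic.
; Light components get temperature or custom color, with intensity zeroed unless BakeLight is set.
; A fixed or random height positions the shade by its mesh bounds, and a spline mesh cable stretches between socket and shade, with per-slot material overrides.
; The TemperatureToColor Kelvin-to-RGB graph is never run.
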(fn `UserConstructionScript`
  (locals (BakeLight_StrenghtSave :type "Float (double-precision)" :default 2000.0) (BakeLight_StrenghtOrigin :type "Float (double-precision)"))
  (bind _lampsocket_mat (`self.Lampsocket_Mat`))
  (bind _lampshade_mat (`self.Lampshade_Mat`))
  (bind _spline_cable (`self.Spline_Cable`))
  (bind _lamp_shade (`self.Lamp_shade`))
  (bind _lamp_socket (`self.Lamp_socket`))
  (bind _light_intensity_internal_use (`self.Light_Intensity_Internal_Use`))
  (bind _lampcable_mat (`self.Lampcable_Mat`))
  (bind (_location _tangent) (`SplineComponent.GetLocationAndTangentAtSplinePoint` _spline_cable 0 "Local"))
  (bind (_location_2 _tangent_2) (`SplineComponent.GetLocationAndTangentAtSplinePoint` _spline_cable 1 "Local"))
  (if (`self.Bake Light`)
    (set `self.Light_Intensity_Internal_Use` (`self.Light Intensity`))
    (else
      (set `self.Light_Intensity_Internal_Use` 0.0)))
  (for _array_element (`self.K2_GetComponentsByClass` "/Script/Engine.LightComponent")
    (if (`LightComponent.bUseTemperature` _array_element)
      (`LightComponent.SetLightColor` _array_element (struct :`R` 0.75 :`G` 0.75 :`B` 0.75 :`A` 1.0) true)
      (`LightComponent.SetTemperature` _array_element (`KismetMathLibrary.Conv_IntToDouble` (`self.Light Temperature`)))
      (`LightComponent.SetIntensity` _array_element _light_intensity_internal_use)
      (else
        (`LightComponent.SetLightColor` _array_element (`self.Light Color`) false)
        (`LightComponent.SetIntensity` _array_element _light_intensity_internal_use)))
    ;[1 1 1] Set Random Height
    (if (`self.Set Random Height`) :!label _label
      (set `self.Lamp Height Internal Use` (`KismetMathLibrary.RandomFloatInRange` (`self.Height Min`) (`self.Height Max`)))
      (else
        (set `self.Lamp Height Internal Use` (`self.Lamp Height`))))
    ;[1 1 1] Set LampSocket
    ;;[1 1 1] Lamp Socket Creation
    (`StaticMeshComponent.SetStaticMesh` _lamp_socket (`self.LampSocket_Input`))
    ;;[1 1 1] Materialslots Lampsocket
    (`KismetArrayLibrary.Array_Resize` _lampsocket_mat (`PrimitiveComponent.GetNumMaterials` _lamp_socket))
    (for (_array_element_2 _array_index) _lampsocket_mat
      (`PrimitiveComponent.SetMaterial` _lamp_socket _array_index _array_element_2)
      ;;[1 1 1] Get Lamp Socket Height
      (set `self.LampSocket_Height` (+ (.z (`SceneComponent.RelativeLocation` _lamp_socket)) (.z (`StaticMeshComponent.GetLocalBounds` _lamp_socket))))
      ;[1 1 1] Set LampShade
      ;;[1 1 1] Lamp Shade Creation
      (`StaticMeshComponent.SetStaticMesh` _lamp_shade (`self.LampShade_Input`))
      ;;[1 1 1] Materialslots Lampshade
      (`KismetArrayLibrary.Array_Resize` _lampshade_mat (`PrimitiveComponent.GetNumMaterials` _lamp_shade))
      (for (_array_element_3 _array_index_2) _lampshade_mat
        (`PrimitiveComponent.SetMaterial` _lamp_shade _array_index_2 _array_element_3)
        (`SceneComponent.K2_SetRelativeLocation` _lamp_shade (`KismetMathLibrary.MakeVector` 0.0 0.0 (- (* (`self.Lamp Height Internal Use`) -1.0) (.z (`StaticMeshComponent.GetLocalBounds` (`self.Lamp_shade`))))) false false)
        ;[1 1 1] Set SplinePoints
        (`SplineComponent.SetLocationAtSplinePoint` (`self.Spline_Cable`) 1 (`KismetMathLibrary.MakeVector` 0.0 0.0 (.z (`StaticMeshComponent.GetLocalBounds` (`self.Lamp_socket`)))) "Local" true)
        (`SplineComponent.SetLocationAtSplinePoint` (`self.Spline_Cable`) 0 (`SceneComponent.RelativeLocation` (`self.Lamp_shade`)) "Local" true)
        ;[1 1 1] Set SplineMesh
        (bind _returnvalue (`AddComponent|NODE_AddSplineMeshComponent-0`))
        (`StaticMeshComponent.SetStaticMesh` _returnvalue (`self.LampCable_Input`))
        (`SceneComponent.K2_AttachTo` _returnvalue (`self.Spline_Cable`) "None" "KeepRelativeOffset" true)
        ;;[1 1 1] Materialslots Lampcable
        (`KismetArrayLibrary.Array_Resize` _lampcable_mat (`PrimitiveComponent.GetNumMaterials` _returnvalue))
        (for (_array_element_4 _array_index_3) _lampcable_mat
          (`PrimitiveComponent.SetMaterial` _returnvalue _array_index_3 _array_element_4)
          (`SplineMeshComponent.SetStartAndEnd` _returnvalue _location _tangent _location_2 _tangent_2 true)))))
  (goto _label))