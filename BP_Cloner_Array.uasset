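; Construction-script cloner actor that lays out an input mesh in a grid of rows and copies using a Hierarchical Instanced Static Mesh.
; Mesh bounds plus configurable gaps set the spacing, and the component shifts by half the X/Y bounds.
; Optional 180° yaw flips alternate copies or rows, with pivot-offset correction from local bounds keeping flipped instances aligned.
; The Z offset is calculated but unused in placement.
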(fn `Calculate Origin Correction`
  (params (Min :type "Vector Structure") (Max :type "Vector Structure"))
  (`/Engine/EditorBlueprintResources/StandardMacros.CompareFloat` Min_X Max_X
    (:`>`
      (bind _returnvalue (`self.Correct for Max A` Min_X Max_X))
      (set `self.Offset X` _returnvalue))
    (:`==`
      _)
    (:`<`
      (bind _returnvalue_2 (`self.Correct for Min A` Max_X Min_X))
      (set `self.Offset X` _returnvalue_2)))
  (`/Engine/EditorBlueprintResources/StandardMacros.CompareFloat` Min_Y Max_Y
    (:`>`
      (bind _returnvalue_3 (`self.Correct for Max A` Min_Y Max_Y))
      (set `self.Offset Y` _returnvalue_3))
    (:`==`
      _)
    (:`<`
      (bind _returnvalue_4 (`self.Correct for Min A` Max_Y Min_Y))
      (set `self.Offset Y` _returnvalue_4)))
  (`/Engine/EditorBlueprintResources/StandardMacros.CompareFloat` Min_Z Max_Z
    (:`>`
      (bind _returnvalue_5 (`self.Correct for Max A` Min_Z Max_Z))
      (set `self.Offset Z` _returnvalue_5))
    (:`==`
      _)
    (:`<`
      (bind _returnvalue_6 (`self.Correct for Min A` Max_Z Min_Z))
      (set `self.Offset Z` _returnvalue_6)))
  (return))

(fn `Correct for Max A`
  (params (`min a` :type "Float (double-precision)") (`max a` :type "Float (double-precision)"))
  (returns (ReturnValue :type "Float (double-precision)"))
  (return (- (/ (+ (* -1 `min a`) `max a`) 2.0) `max a`)))

(fn `Correct for Min A`
  (params (`min a` :type "Float (double-precision)") (`max a` :type "Float (double-precision)"))
  (returns (ReturnValue :type "Float (double-precision)"))
  (bind _returnvalue (* -1 `min a`))
  (return (- (/ (+ _returnvalue `max a`) 2.0) _returnvalue)))

(fn `UserConstructionScript`
  (bind _hierarchicalinstancedstaticmesh (`self.HierarchicalInstancedStaticMesh`))
  (bind _hierarchicalinstancedstaticmesh_2 (`self.HierarchicalInstancedStaticMesh`))
  (bind (_min _max) (`StaticMeshComponent.GetLocalBounds` (`self.HierarchicalInstancedStaticMesh`)))
  (bind (_x_bound _y_bound) (`/Game/blueprints/BPL_CommonMacros.Get Combined Bounds` (`self.HierarchicalInstancedStaticMesh`)))
  (bind (_x_bound_2 _y_bound_2) (`/Game/blueprints/BPL_CommonMacros.Get Combined Bounds` _hierarchicalinstancedstaticmesh))
  ;[1 1 1] Create Mesh (Instanced)
  (`StaticMeshComponent.SetStaticMesh` _hierarchicalinstancedstaticmesh_2 (`self.Input Mesh`))
  (`SceneComponent.K2_SetRelativeTransform` _hierarchicalinstancedstaticmesh_2 (`KismetMathLibrary.MakeTransform` (0.0 0.0 0.0) (struct) (`self.Mesh Scale`)) false false)
  ;[1 1 1] Calculate Mesh Origin Correction
  (`self.Calculate Origin Correction` _min _max)
  (`SceneComponent.K2_SetRelativeTransform` _hierarchicalinstancedstaticmesh (`KismetMathLibrary.MakeTransform` (`KismetMathLibrary.MakeVector` (/ _x_bound_2 2.0) (/ _y_bound_2 2.0))) false false)
  (for _index (range (`self.Number Of Rows`))
    (for _index_2 (range (`self.Number Of Copys`))
      (bind _returnvalue (* _index_2 (+ _x_bound (`self.Distance Between Copys`))))
      (bind _returnvalue_2 (`KismetMathLibrary.Lerp` 1.0 -1.0 (* (`KismetMathLibrary.Conv_IntToDouble` (mod _index 2)) (`KismetMathLibrary.Conv_BoolToDouble` (`self.Rotate Rows 180°`)))))
      (bind _returnvalue_3 (* _index (+ _y_bound (`self.Distance Between Rows`))))
      (bind _returnvalue_4 (`KismetMathLibrary.Conv_IntToDouble` (mod (* _index_2 (`KismetMathLibrary.Conv_BoolToInt` (`self.Rotate Copys 180°`))) 2)))
      (bind (_returnvalue_roll _returnvalue_pitch _returnvalue_yaw) (`KismetMathLibrary.BreakRotator` (`KismetMathLibrary.RLerp` (struct) (struct :`Yaw` 180.0) (`KismetMathLibrary.Conv_IntToDouble` (mod (* _index (`KismetMathLibrary.Conv_BoolToInt` (`self.Rotate Rows 180°`))) 2)))))
      (`InstancedStaticMeshComponent.AddInstance` (`self.HierarchicalInstancedStaticMesh`) (`KismetMathLibrary.MakeTransform` (`KismetMathLibrary.VLerp` (`KismetMathLibrary.MakeVector` (+ _returnvalue (* (`self.Offset X`) _returnvalue_2)) (+ _returnvalue_3 (`self.Offset Y`))) (`KismetMathLibrary.MakeVector` (- _returnvalue (* (`self.Offset X`) _returnvalue_2)) (- _returnvalue_3 (`self.Offset Y`))) _returnvalue_4) (`KismetMathLibrary.RLerp` (`KismetMathLibrary.MakeRotator` 0.0 0.0 (+ 180.0 _returnvalue_yaw)) (`KismetMathLibrary.MakeRotator` 0.0 0.0 _returnvalue_yaw) _returnvalue_4))))))