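; Procedural door generator that assembles a sized frame, leaf, handle and hinges from input meshes in the Construction Script, with no runtime logic.
; Frame pieces and leaf are positioned or stretched from mesh bounds to fit dimensions given in centimetres or taken from actor scale.
; CounterRootScaling helpers compensate for root scale, and hinges are spaced evenly along one side.
; Leaf and handle attach to a hinge pivot, yawed by OpenByDegrees to pose the door open.
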(fn `IsScaleForWidthActivated?`
  (bind _returnvalue_x (`KismetMathLibrary.BreakVector` (`SceneComponent.K2_GetComponentScale` (`self.DefaultSceneRoot`))))
  (bind (_returnvalue_x_2 _returnvalue_y _returnvalue_z) (`KismetMathLibrary.BreakVector` (`SceneComponent.K2_GetComponentScale` (`self.DefaultSceneRoot`))))
  (bind _returnvalue_x_3 (`KismetMathLibrary.BreakVector` (`SceneComponent.K2_GetComponentScale` (`self.DefaultSceneRoot`))))
  (if (`self.Use Scale For Width`)
    (set `self.Scale For Width Enabled?` 1.0)
    (set `self.DoorWidth in cm` (`self.Counter RootScaling X` (* _returnvalue_x_3 100.0)))
    (set `self.DoorHeight in cm` (`self.Counter RootScaling Z` (* _returnvalue_z 100.0)))
    (else
      (set `self.Scale For Width Enabled?` (/ 1.0 _returnvalue_x)))))

(fn `Set And Place Door Hinges`
  (bind _returnvalue (* (- (- (/ (`self.DoorFinalWidth`) 2.0) (`self.Add Up X Bounds` (`self.DoorSide1`))) (`self.Counter RootScaling X` (* (`self.HingePlacementX`) -1.0))) -1.0))
  (for _index (range (`self.Hinge Number`))
    (bind _returnvalue_2 (`AddComponent|NODE_AddStaticMeshComponent-18`))
    (`StaticMeshComponent.SetStaticMesh` _returnvalue_2 (`self.DoorHingeInput`))
    (bind _returnvalue_3 (+ (.y (`.Max` (`StaticMeshComponent.GetLocalBounds` (`self.DoorSide1`)))) (* (.y (`StaticMeshComponent.GetLocalBounds` _returnvalue_2)) -1.0)))
    (`SceneComponent.K2_SetRelativeLocation` _returnvalue_2 (`KismetMathLibrary.MakeVector` _returnvalue _returnvalue_3 (+ (* (`self.DoorHingeZPlacement`) (`KismetMathLibrary.Conv_IntToDouble` _index)) (`self.Counter RootScaling Z` (`self.HingePlacementZ`)))) false false)
    (`SceneComponent.SetRelativeScale3D` _returnvalue_2 (`KismetMathLibrary.MakeVector` (`self.Counter RootScaling X` 1.0) 1.0 (`self.Counter RootScaling Z` 1.0))))
  (set `self.HingeLocationXY` (`KismetMathLibrary.MakeVector2D` _returnvalue _returnvalue_3)))

(fn `SetDoorCorner Meshs`
  (params (DoorSideMesh1 :type "StaticMesh Object Reference") (DoorSideMesh2 :type "StaticMesh Object Reference"))
  (bind _returnvalue (`AddComponent|NODE_AddStaticMeshComponent-10`))
  (bind _output_get (set `self.DoorCorner1` _returnvalue))
  (`StaticMeshComponent.SetStaticMesh` _output_get DoorSideMesh2)
  (`SceneComponent.K2_SetRelativeTransform` _output_get (`KismetMathLibrary.MakeTransform` (0.0 0.0 0.0) (struct) (`KismetMathLibrary.MakeVector` (`self.Counter RootScaling X` 1.0) 1.0 (`self.Counter RootScaling Z` 1.0))) false false)
  (bind _returnvalue_2 (`AddComponent|NODE_AddStaticMeshComponent-9`))
  (bind _output_get_2 (set `self.DoorCorner2` _returnvalue_2))
  (`StaticMeshComponent.SetStaticMesh` _output_get_2 DoorSideMesh1)
  (`SceneComponent.K2_SetRelativeTransform` _output_get_2 (`KismetMathLibrary.MakeTransform` (0.0 0.0 0.0) (struct) (`KismetMathLibrary.MakeVector` (`self.Counter RootScaling X` -1.0) 1.0 (`self.Counter RootScaling Z` 1.0))) false false))

(fn `SetDoorHandle Mesh`
  (params (NewMesh :type "StaticMesh Object Reference"))
  (bind _returnvalue (`AddComponent|NODE_AddStaticMeshComponent-14`))
  (bind _output_get (set `self.DoorHandle` _returnvalue))
  (`StaticMeshComponent.SetStaticMesh` _output_get NewMesh)
  (`SceneComponent.K2_SetRelativeTransform` _returnvalue (`KismetMathLibrary.MakeTransform` (0.0 0.0 0.0) (struct) (`KismetMathLibrary.MakeVector` (`self.Counter RootScaling X` 1.0) 1.0 (`self.Counter RootScaling Z` 1.0))) false false))

(fn `SetDoorHandlePosition`
  (bind (_min _max) (`StaticMeshComponent.GetLocalBounds` (`self.DoorLeaf`)))
  (`SceneComponent.K2_SetRelativeLocation` (`self.DoorHandle`) (`KismetMathLibrary.MakeVector` (- (/ (- (`self.DoorFinalWidth`) (* (`self.Counter RootScaling X` (.x (`StaticMeshComponent.GetLocalBounds` (`self.DoorSide1`)))) -2.0)) 2.0) (`self.Counter RootScaling X` (`self.HandleDistance`))) (/ (+ (.y _min) (.y _max)) 2.0) (`self.Counter RootScaling Z` (`self.HandleHeight`))) false false))

(fn `SetDoorHeightBounds`
  (bind _doortop (`self.DoorTop`))
  (bind _doorside1 (`self.DoorSide1`))
  (bind _doorside2 (`self.DoorSide2`))
  (bind _doorcorner1 (`self.DoorCorner1`))
  (bind _doorcorner2 (`self.DoorCorner2`))
  (bind (_relativelocation_x _relativelocation_y) (`KismetMathLibrary.BreakVector` (`SceneComponent.RelativeLocation` _doorcorner1)))
  (bind (_relativelocation_x_2 _relativelocation_y_2) (`KismetMathLibrary.BreakVector` (`SceneComponent.RelativeLocation` _doortop)))
  (bind (_relativelocation_x_3 _relativelocation_y_3) (`KismetMathLibrary.BreakVector` (`SceneComponent.RelativeLocation` _doorcorner2)))
  (bind (_relativescale3d_x _relativescale3d_y) (`KismetMathLibrary.BreakVector` (`SceneComponent.RelativeScale3D` _doorside2)))
  (bind (_relativescale3d_x_2 _relativescale3d_y_2) (`KismetMathLibrary.BreakVector` (`SceneComponent.RelativeScale3D` _doorside1)))
  (bind _returnvalue (- (`self.DoorFinalHeight`) (`self.Counter RootScaling Z` (.z (`.Max` (`StaticMeshComponent.GetLocalBounds` (`self.DoorCorner1`)))))))
  (bind _returnvalue_2 (* 1.0 (/ (- (`self.DoorFinalHeight`) (`self.DoorCornerHeight`)) (.z (`.Max` (`StaticMeshComponent.GetLocalBounds` _doorside1))))))
  ;[1 1 1] Set Door Corner Height Positions
  (`SceneComponent.K2_SetRelativeLocation` _doorcorner1 (`KismetMathLibrary.MakeVector` _relativelocation_x _relativelocation_y _returnvalue) false false)
  (`SceneComponent.K2_SetRelativeLocation` _doorcorner2 (`KismetMathLibrary.MakeVector` _relativelocation_x_3 _relativelocation_y_3 _returnvalue) false false)
  (`SceneComponent.K2_SetRelativeLocation` _doortop (`KismetMathLibrary.MakeVector` _relativelocation_x_2 _relativelocation_y_2 _returnvalue) false false)
  ;[1 1 1] Scale DoorSide
  (`SceneComponent.SetRelativeScale3D` _doorside1 (`KismetMathLibrary.MakeVector` _relativescale3d_x_2 _relativescale3d_y_2 _returnvalue_2))
  (`SceneComponent.SetRelativeScale3D` _doorside2 (`KismetMathLibrary.MakeVector` _relativescale3d_x _relativescale3d_y _returnvalue_2)))

(fn `SetDoorHinge Mesh`
  (params (self2 :type "StaticMesh Object Reference"))
  (bind _returnvalue (`AddComponent|NODE_AddStaticMeshComponent-17`))
  (bind _output_get (set `self.DoorHinge` _returnvalue))
  (`StaticMeshComponent.SetStaticMesh` _output_get self2)
  (`SceneComponent.K2_SetRelativeTransform` _returnvalue (`KismetMathLibrary.MakeTransform` (0.0 0.0 0.0) (struct) (1.0 1.0 1.0)) false false))

(fn `SetDoorHingeDistanceZ`
  (set `self.DoorHingeZPlacement` (/ (- (- (`self.DoorFinalHeight`) (`self.Add Up Z Bounds` (`self.DoorTop`))) (`self.Counter RootScaling Z` (* (`self.HingePlacementZ`) 2.0))) (`KismetMathLibrary.Conv_IntToDouble` (- (`self.Hinge Number`) 1)))))

(fn `SetDoorLeaf Mesh`
  (params (NewMesh :type "StaticMesh Object Reference"))
  (bind _returnvalue (`AddComponent|NODE_AddStaticMeshComponent-16`))
  (bind _output_get (set `self.DoorLeaf` _returnvalue))
  (`StaticMeshComponent.SetStaticMesh` _output_get NewMesh)
  (`SceneComponent.K2_SetRelativeTransform` _output_get (`KismetMathLibrary.MakeTransform` (0.0 0.0 0.0) (struct) (`KismetMathLibrary.MakeVector` (`self.Counter RootScaling X` 1.0) 1.0 (`self.Counter RootScaling Z` 1.0))) false false))

(fn `SetDoorLeafTransform`
  (bind _hingelocationxy_x (`KismetMathLibrary.BreakVector2D` (`self.HingeLocationXY`)))
  (bind _hingelocationxy_x_2 (`KismetMathLibrary.BreakVector2D` (`self.HingeLocationXY`)))
  (bind _hingelocationxy_x_3 (`KismetMathLibrary.BreakVector2D` (`self.HingeLocationXY`)))
  (`SceneComponent.K2_SetRelativeTransform` (`self.DoorLeaf`) (`KismetMathLibrary.MakeTransform` (`KismetMathLibrary.MakeVector` (- _hingelocationxy_x_2 (* (.x (`.BoxExtent` (`KismetMathLibrary.BreakBoxSphereBounds` (`StaticMesh.GetBounds` (`self.DoorHingeInput`))))) -1.0))) (`KismetMathLibrary.MakeRotator` 0.0) (`KismetMathLibrary.MakeVector` (* 1.0 (/ (- (* _hingelocationxy_x_3 -1.0) (.x (`.Max` (`StaticMeshComponent.GetLocalBounds` (`self.DoorHinge`))))) (/ (`self.Add Up X Bounds` (`self.DoorLeaf`)) 2.0))) 1.0 (* 1.0 (/ (- (`self.DoorFinalHeight`) (`self.Counter RootScaling Z` (- (/ (`self.DoorFinalWidth`) 2.0) (- (* _hingelocationxy_x -1.0) (.z (`.Max` (`StaticMeshComponent.GetLocalBounds` (`self.DoorHinge`)))))))) (`self.Add Up Z Bounds` (`self.DoorLeaf`)))))) false false))

(fn `SetDoorSide Meshs`
  (params (DoorSideMesh1 :type "StaticMesh Object Reference") (DoorSideMesh2 :type "StaticMesh Object Reference"))
  (bind _returnvalue (`AddComponent|NODE_AddStaticMeshComponent-8`))
  (bind _output_get (set `self.DoorSide1` _returnvalue))
  (`StaticMeshComponent.SetStaticMesh` _output_get DoorSideMesh2)
  (`SceneComponent.K2_SetRelativeTransform` _output_get (`KismetMathLibrary.MakeTransform` (0.0 0.0 0.0) (struct) (`KismetMathLibrary.MakeVector` (`self.Counter RootScaling X` 1.0) 1.0 (`self.Counter RootScaling Z` 1.0))) false false)
  (bind _returnvalue_2 (`AddComponent|NODE_AddStaticMeshComponent-7`))
  (bind _output_get_2 (set `self.DoorSide2` _returnvalue_2))
  (`StaticMeshComponent.SetStaticMesh` _output_get_2 DoorSideMesh1)
  (`SceneComponent.K2_SetRelativeTransform` _output_get_2 (`KismetMathLibrary.MakeTransform` (0.0 0.0 0.0) (struct) (`KismetMathLibrary.MakeVector` (`self.Counter RootScaling X` -1.0) 1.0 (`self.Counter RootScaling Z` 1.0))) false false))

(fn `SetDoorTop Mesh`
  (params (DoorTopMesh :type "StaticMesh Object Reference"))
  (bind _returnvalue (`AddComponent|NODE_AddStaticMeshComponent-13`))
  (bind _output_get (set `self.DoorTop` _returnvalue))
  (`StaticMeshComponent.SetStaticMesh` _output_get DoorTopMesh)
  (`SceneComponent.K2_SetRelativeTransform` _output_get (`KismetMathLibrary.MakeTransform` (0.0 0.0 0.0) (struct) (`KismetMathLibrary.MakeVector` (`self.Counter RootScaling X` 1.0) 1.0 (`self.Counter RootScaling Z` 1.0))) false false))

(fn `SetDoorWidthBounds`
  (bind _doortop (`self.DoorTop`))
  (bind _doorside1 (`self.DoorSide1`))
  (bind _doorside2 (`self.DoorSide2`))
  (bind _doorcorner1 (`self.DoorCorner1`))
  (bind _doorcorner2 (`self.DoorCorner2`))
  (bind (_relativescale3d_x _relativescale3d_y _relativescale3d_z) (`KismetMathLibrary.BreakVector` (`SceneComponent.RelativeScale3D` _doortop)))
  (bind (_relativelocation_x _relativelocation_y _relativelocation_z) (`KismetMathLibrary.BreakVector` (`SceneComponent.RelativeLocation` _doorcorner2)))
  (bind (_relativelocation_x_2 _relativelocation_y_2 _relativelocation_z_2) (`KismetMathLibrary.BreakVector` (`SceneComponent.RelativeLocation` _doorside1)))
  (bind (_relativelocation_x_3 _relativelocation_y_3 _relativelocation_z_3) (`KismetMathLibrary.BreakVector` (`SceneComponent.RelativeLocation` _doorside2)))
  (bind (_relativelocation_x_4 _relativelocation_y_4 _relativelocation_z_4) (`KismetMathLibrary.BreakVector` (`SceneComponent.RelativeLocation` _doorcorner1)))
  (bind _returnvalue (- (/ (`self.DoorFinalWidth`) 2.0) (`self.Counter RootScaling X` (* (.x (`StaticMeshComponent.GetLocalBounds` (`self.DoorCorner1`))) -1.0))))
  (bind _returnvalue_2 (* _returnvalue -1.0))
  ;[1 1 1] Set Door Side Positions
  (`SceneComponent.K2_SetRelativeLocation` _doorside1 (`KismetMathLibrary.MakeVector` _returnvalue_2 _relativelocation_y_2 _relativelocation_z_2) false false)
  (`SceneComponent.K2_SetRelativeLocation` _doorside2 (`KismetMathLibrary.MakeVector` _returnvalue _relativelocation_y_3 _relativelocation_z_3) false false)
  (`SceneComponent.K2_SetRelativeLocation` _doorcorner1 (`KismetMathLibrary.MakeVector` _returnvalue_2 _relativelocation_y_4 _relativelocation_z_4) false false)
  (`SceneComponent.K2_SetRelativeLocation` _doorcorner2 (`KismetMathLibrary.MakeVector` _returnvalue _relativelocation_y _relativelocation_z) false false)
  ;[1 1 1] Scale DoorTop
  (`SceneComponent.SetRelativeScale3D` _doortop (`KismetMathLibrary.MakeVector` (* (* 1.0 (/ (- (`self.DoorFinalWidth`) (* (`self.DoorCornerWidth`) 2.0)) (* (.x (`StaticMeshComponent.GetLocalBounds` _doortop)) 2.0))) -1.0) _relativescale3d_y _relativescale3d_z)))

(fn `UserConstructionScript`
  (bind _rotationempty (`self.RotationEmpty`))
  (bind _doorleaf (`self.DoorLeaf`))
  (bind (_hingelocationxy_x _hingelocationxy_y) (`KismetMathLibrary.BreakVector2D` (`self.HingeLocationXY`)))
  (bind _hingelocationxy_x_2 (`KismetMathLibrary.BreakVector2D` (`self.HingeLocationXY`)))
  (bind _doorsideinput (`self.DoorSideInput`))
  (bind _doorcornerinput (`self.DoorCornerInput`))
  (bind (_relativescale3d_x _relativescale3d_y _relativescale3d_z) (`KismetMathLibrary.BreakVector` (`SceneComponent.RelativeScale3D` _doorleaf)))
  (bind (_relativelocation_x _relativelocation_y _relativelocation_z) (`KismetMathLibrary.BreakVector` (`SceneComponent.RelativeLocation` _doorleaf)))
  ;[1 0 0] Booleans
  (`self.IsScaleForWidthActivated?`)
  ;[1 0.4824 0.8863] 1. Set Final Width
  (`self.Set Door Final Width`)
  ;[1 0.4824 0.8863] 2. Set Final Height
  (`self.Set Door Final Height`)
  ;[1 1 1] 3. Set Hinge Distance Z
  (`self.SetDoorHingeDistanceZ`)
  ;[0 0.3086 1] 4. Set Meshes
  (`self.SetDoorTop Mesh` (`self.DoorTopInput`))
  (`self.SetDoorSide Meshs` _doorsideinput _doorsideinput)
  (`self.SetDoorCorner Meshs` _doorcornerinput _doorcornerinput)
  (`self.SetDoorLeaf Mesh` (`self.DoorLeafInput`))
  (`self.SetDoorHandle Mesh` (`self.DoorHandleInput`))
  (`self.Set And Place Door Hinges`)
  (set `self.DoorCornerWidth` (`self.Add Up X Bounds` (`self.DoorCorner1`)))
  (set `self.DoorCornerHeight` (`self.Add Up Z Bounds` (`self.DoorCorner1`)))
  (`self.SetDoorWidthBounds`)
  (`self.SetDoorHeightBounds`)
  (`self.SetDoorLeafTransform`)
  (`self.SetDoorHandlePosition`)
  ;[1 1 1] Comment
  (if (`self.Use Scale For Width`)
    (`SceneComponent.SetRelativeScale3D` _doorleaf (`KismetMathLibrary.MakeVector` (`self.Counter RootScaling X` _relativescale3d_x) _relativescale3d_y (`self.Counter RootScaling Z` _relativescale3d_z)))
    (`SceneComponent.K2_SetRelativeLocation` _doorleaf (`KismetMathLibrary.MakeVector` (- _hingelocationxy_x_2 (`self.Counter RootScaling X` (.x (break `Box` (`StaticMesh.GetBoundingBox` (`self.DoorHingeInput`)))))) _relativelocation_y _relativelocation_z) false false))
  ;[1 1 1] Comment
  (`SceneComponent.K2_SetRelativeLocation` (`self.RotationEmpty`) (`KismetMathLibrary.MakeVector` _hingelocationxy_x _hingelocationxy_y) false false)
  ;[1 1 1] Parent Handle To Hinge
  (`SceneComponent.K2_AttachToComponent` (`self.DoorHandle`) _rotationempty "None" "KeepWorld" "KeepRelative" "KeepWorld" true)
  ;[1 1 1] Parent Leaf To Hinge
  (`SceneComponent.K2_AttachToComponent` (`self.DoorLeaf`) _rotationempty "None" "KeepWorld" "KeepRelative" "KeepWorld" true)
  (`SceneComponent.K2_SetRelativeRotation` _rotationempty (`KismetMathLibrary.MakeRotator` 0.0 0.0 (`self.OpenByDegrees`)) false false))