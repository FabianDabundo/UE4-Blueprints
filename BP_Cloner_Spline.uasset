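; Spline-based cloner actor that places copies of a static mesh along a spline in the construction script.
; CopyType selects either fixed Spacing or a fixed Number spread over the spline length.
; Copies optionally follow spline rotation, and RandomizeRotation adds weighted per-axis random rotation to each.
; A separate EndMesh snaps to the spline end; non-following Fixed Number copies also scale their position by the Offset-adjusted tangent.
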(fn `UserConstructionScript`
  (bind _spline (`self.Spline`))
  (bind (_endmeshrotation_roll _endmeshrotation_pitch _endmeshrotation_yaw) (`KismetMathLibrary.BreakRotator` (`self.EndMeshRotation`)))
  (bind _spline_2 (`self.Spline`))
  (bind _spline_3 (`self.Spline`))
  (bind _spline_4 (`self.Spline`))
  (bind _returnvalue (- (`self.Number`) 1))
  (bind _returnvalue_2 (`SplineComponent.GetNumberOfSplinePoints` _spline))
  (bind (_returnvalue_roll _returnvalue_pitch _returnvalue_yaw) (`KismetMathLibrary.BreakRotator` (`SplineComponent.GetRotationAtSplinePoint` _spline _returnvalue_2 "World")))
  (`StaticMeshComponent.SetStaticMesh` (`self.EndMesh`) (`self.EndMeshInput`))
  (set `self.CopyMeshRotationInternal` (`KismetMathLibrary.ComposeRotators` (`self.CopyMeshRotationInternal`) (`self.CopyMeshRotation`)))
  (switch `/Game/blueprints/E_Cloner_Spline` (`self.Copy Type`)
    (:`NewEnumerator0`
      ;[1 1 1] Copy Mesh Spacing
      (for _index (range (+ (`.ReturnValue` (`KismetMathLibrary.FMod` (`SplineComponent.GetSplineLength` (`self.Spline`)) (`self.Spacing`))) 1))
        (if (`self.RotationFollowsSpline`)
          ;[1 1 1] Randomize Rotation
          (`self.Randomize Rotation`)
          (bind _returnvalue_3 (* _index (`self.Spacing`)))
          (bind _returnvalue_4 (`AddComponent|NODE_AddStaticMeshComponent-0` :`bManualAttachment` true :`RelativeTransform` (`KismetMathLibrary.MakeTransform` (`SplineComponent.GetLocationAtDistanceAlongSpline` _spline_3 _returnvalue_3 "World") (`KismetMathLibrary.ComposeRotators` (`SplineComponent.GetRotationAtDistanceAlongSpline` _spline_3 _returnvalue_3 "World") (`self.CopyMeshRotationInternal`)))))
          (`StaticMeshComponent.SetStaticMesh` _returnvalue_4 (`self.CopyMeshInput`))
          (else
            ;[1 1 1] Randomize Rotation
            (`self.Randomize Rotation`)
            (bind _returnvalue_5 (`AddComponent|NODE_AddStaticMeshComponent-3` :`bManualAttachment` true :`RelativeTransform` (`KismetMathLibrary.MakeTransform` (`SplineComponent.GetLocationAtDistanceAlongSpline` (`self.Spline`) _returnvalue_3 "World") (`self.CopyMeshRotationInternal`))))
            (`StaticMeshComponent.SetStaticMesh` _returnvalue_5 (`self.CopyMeshInput`))))
        ;[1 1 1] Add EndMesh
        (`SceneComponent.K2_SetRelativeLocationAndRotation` (`self.EndMesh`) (`SplineComponent.GetLocationAtSplinePoint` _spline _returnvalue_2 "Local") (`KismetMathLibrary.MakeRotator` _endmeshrotation_roll (+ _returnvalue_pitch _endmeshrotation_pitch) (+ _returnvalue_yaw _endmeshrotation_yaw)) false false :!label _label)))
    (:`NewEnumerator1`
      ;[1 1 1] Copy Mesh Fixed Number
      (for _index_2 (range (+ _returnvalue 1))
        (if (`self.RotationFollowsSpline`)
          ;[1 1 1] Randomize Rotation
          (`self.Randomize Rotation`)
          (bind _returnvalue_6 (* _index_2 (/ (`SplineComponent.GetSplineLength` (`self.Spline`)) (`KismetMathLibrary.Conv_IntToDouble` _returnvalue))))
          (bind _returnvalue_7 (`AddComponent|NODE_AddStaticMeshComponent-1` :`bManualAttachment` true :`RelativeTransform` (`KismetMathLibrary.MakeTransform` (`SplineComponent.GetLocationAtDistanceAlongSpline` _spline_2 _returnvalue_6 "World") (`KismetMathLibrary.ComposeRotators` (`SplineComponent.GetRotationAtDistanceAlongSpline` _spline_2 _returnvalue_6 "World") (`self.CopyMeshRotationInternal`)))))
          (`StaticMeshComponent.SetStaticMesh` _returnvalue_7 (`self.CopyMeshInput`))
          (goto _label)
          (else
            ;[1 1 1] Randomize Rotation
            (`self.Randomize Rotation`)
            (bind (_returnvalue_x _returnvalue_y _returnvalue_z) (`KismetMathLibrary.BreakVector` (`KismetMathLibrary.Normal` (`SplineComponent.GetTangentAtDistanceAlongSpline` _spline_4 _returnvalue_6 "Local"))))
            (bind _returnvalue_8 (`AddComponent|NODE_AddStaticMeshComponent-2` :`bManualAttachment` true :`RelativeTransform` (`KismetMathLibrary.MakeTransform` (* (`KismetMathLibrary.MakeVector` (+ _returnvalue_x (`self.Offset`)) _returnvalue_y _returnvalue_z) (`SplineComponent.GetLocationAtDistanceAlongSpline` _spline_4 _returnvalue_6 "World")) (`self.CopyMeshRotationInternal`))))
            (`StaticMeshComponent.SetStaticMesh` _returnvalue_8 (`self.CopyMeshInput`))
            (goto _label)))))))